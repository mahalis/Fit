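; ObstacleRing is a ring actor that tests whether the pins of another ring fit it at their current relative rotation.
; CheckPins takes the pin ring's first data entry's hole indices plus index zero, shifts each by both rings' segment offsets and the pin shift, wraps by segment count, and looks up matching segments.
; It reports whether all pins fit, with a count that drops to zero on any misfit.
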(event EventBeginPlay
  (|CallParentFunction) ; This node is disabled and will not be called.\nDrag off pins to build functionality.
)

(event Collision|EventActorBeginOverlap
  (params (OtherActor :type Actor%20Object%20Reference))
  (|CallParentFunction OtherActor) ; This node is disabled and will not be called.\nDrag off pins to build functionality.
)

(event EventTick
  (params (DeltaSeconds :type Float%20%28single-precision%29))
  (|CallParentFunction DeltaSeconds) ; This node is disabled and will not be called.\nDrag off pins to build functionality.
)

(fn ConstructionScript
  (|CallParentFunction))

(fn CheckPins
  (params (PinRing :type Pin%20Ring%20Object%20Reference))
  (bind _alldata (Variables|/Game/Blueprints/ThingRing.ThingRing_C|GetAllData PinRing))
  (bind _output (Utilities|Array|Get(acopy) _alldata))
  (bind _output_get (LocalVariables|SetFullPinIndices (.holeindices _output)))
  (Utilities|Array|Add _output_get 0)
  (for _array_element (LocalVariables|GetFullPinIndices)
    (bind _has (CallFunction|AnyRingDataHasSegment (Math|Integer|%(Integer) (Utilities|Operators|Subtract (+ (.RealSegmentOffset (Default|State (Variables|Default|GetRotationComponent))) _array_element) (Variables|/Game/Blueprints/RotationComponent.RotationComponent_C|GetSegmentOffset (Variables|/Game/Blueprints/ThingRing.ThingRing_C|GetRotationComponent PinRing)) (.pinshiftamount _output)) (Variables|/Game/Blueprints/RotationComponent.RotationComponent_C|GetSegmentCount (Variables|Default|GetRotationComponent)))))
    (if _has
      (Math|Integer|IncrementInt (LocalVariables|GetFitCount))
      (else
        (LocalVariables|SetFoundAnyMisfits true))))
  (return (not (LocalVariables|GetFoundAnyMisfits)) (Math|Integer|SelectInt 0 (LocalVariables|GetFitCount) (LocalVariables|GetFoundAnyMisfits))))