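; ThingRing is a rotating segmented ring actor whose visible segments reflect an array of ring data with pin shifts and hole indices.
; The construction script builds segment meshes around SegmentRoot, with optional rect lights and a random starting offset.
; A segment matching any entry's shifted zero position or holes is hidden, or shown when VisibilityInverted.
; RotationComponent handles moves and offsets, and Tick applies its angle to SegmentRoot.
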(event EventBeginPlay)

(event Collision|EventActorBeginOverlap
  (params (OtherActor :type Actor%20Object%20Reference)))

(event EventTick
  (params (DeltaSeconds :type Float%20%28single-precision%29))
  (CallFunction|UpdateRotation))

(fn ConstructionScript
  (bind _rotationcomponent (Variables|Default|GetRotationComponent))
  (bind _segmentcount (Variables|/Game/Blueprints/RotationComponent.RotationComponent_C|GetSegmentCount _rotationcomponent))
  (bind _returnvalue (- _segmentcount 1))
  (if (Variables|Default|GetRandomizeStartingOffset)
    (Default|SetOffsetInstant (Variables|Default|GetRotationComponent) (Math|Random|RandomIntegerinRange 0 _returnvalue)))
  (for _index (range 0 _returnvalue)
    (bind _returnvalue_2 (AddComponent|AddStaticMeshComponent true (Math|Transform|MakeTransform "0, 0, 0" (Math|Rotator|MakeRotator 0.0 (+ (* (/ (Math|Conversions|ToFloat(Integer) _index) _segmentcount) 3.6e+02) -9e+01) 0.0) "1.000000,1.000000,1.000000")))
    (Transformation|AttachComponentToComponent _returnvalue_2 (Variables|Default|GetSegmentRoot) "None" "KeepRelative" "KeepRelative" "SnapToTarget" true)
    (Components|StaticMesh|SetStaticMesh _returnvalue_2 (Variables|Default|GetSegmentMesh))
    (Utilities|Array|Add (Variables|Default|GetSegmentMeshes) _returnvalue_2)
    (if (Variables|Default|GetWantsSegmentLights)
      (bind _returnvalue_3 (AddComponent|AddRectLightComponent false (Math|Transform|MakeTransform (Math|Vector|RotateVectorAroundAxis "0.000000,190.000000,0.000000" (+ (* (/ (Math|Conversions|ToFloat(Integer) _index) _segmentcount) 3.6e+02) -9e+01) "1.000000,0.000000,0.000000") "0.000000,90.000000,90.000000" "1.000000,1.000000,1.000000")))
      (Transformation|AttachComponentToComponent _returnvalue_3 _returnvalue_2 "None" "KeepWorld" "KeepRelative" "KeepRelative" true)
      (Utilities|Array|Add (Variables|Default|GetSegmentLights) _returnvalue_3)))
  (CallFunction|UpdatefromData))

(fn SetRingState
  (params (AllData :type Array%20of%20Segment%20Data%20Structures) (Offset :type Integer))
  (Variables|Default|SetAllData AllData)
  (Default|SetOffsetInstant (Variables|Default|GetRotationComponent) Offset)
  (CallFunction|UpdatefromData))

(fn UpdatefromData
  (for (_array_element _array_index) (Variables|Default|GetSegmentMeshes)
    (bind _has (CallFunction|AnyRingDataHasSegment _array_index))
    (Rendering|SetVisibility _array_element (== _has (Variables|Default|GetVisibilityInverted)) true)))

(fn Move
  (params (Right :type Boolean))
  (Default|Move (Variables|Default|GetRotationComponent) Right))

(fn UpdateRotation
  (Transformation|SetRelativeRotation (Variables|Default|GetSegmentRoot) (Math|Rotator|MakeRotator 0.0 (.Degrees (Default|State (Variables|Default|GetRotationComponent))) 9e+01) false false))

(fn AnyRingDataHasSegment
  (params (SegmentIndex :type Integer))
  (bind _rotationcomponent (Variables|Default|GetRotationComponent))
  (bind _segmentcount (Variables|/Game/Blueprints/RotationComponent.RotationComponent_C|GetSegmentCount _rotationcomponent))
  (for (_array_element _array_index) (Variables|Default|GetAllData)
    (if (or (== (Math|Integer|%(Integer) (+ SegmentIndex (.PinShiftAmount (Utilities|Struct|BreakSegmentData _array_element)) _segmentcount) _segmentcount) 0) (Utilities|Array|ContainsItem (.HoleIndices (Utilities|Struct|BreakSegmentData _array_element)) (Math|Integer|%(Integer) (+ SegmentIndex (.PinShiftAmount (Utilities|Struct|BreakSegmentData _array_element)) _segmentcount) _segmentcount)))
      (return true)))
  (return false))