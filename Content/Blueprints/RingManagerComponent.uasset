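; Manager component that runs a scrolling ring puzzle, where the player's pin ring must fit through oncoming obstacle rings.
; Each tick it slides obstacles along -X past the near-stationary player, destroys those far behind, and spawns random replacements ahead.
; The first ring still ahead in the ordered list becomes the active incoming ring.
; MovePlayerPins moves the pin ring and checks it against that ring, showing debug-shape feedback only.
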(event EventBeginPlay
  (Utilities|FlowControl|Sequence
    (:then_0
      (bind _returnvalue (Game|SpawnActorfromClass "/Game/Blueprints/ObstacleRing.ObstacleRing_C" (Math|Transform|MakeTransform "0, 0, 0" "0, 0, 0" "1.000000,1.000000,1.000000") "AlwaysSpawn" "MultiplyWithRoot" 0 (.OutItem (Utilities|Array|Random (Variables|Default|GetAvailableRings))) true 0))
      (bind _output_get (Variables|Default|SetActiveIncomingRing _returnvalue))
      (Utilities|Array|Add (Variables|Default|GetObstacleRings) _output_get))
    (:then_1
      (bind _returnvalue_2 (Game|SpawnActorfromClass "/Game/Blueprints/PinRing.PinRing_C" (Math|Transform|MakeTransform "-5.000000,0.000000,0.000000" "0, 0, 0" "1.000000,1.000000,1.000000") "AlwaysSpawn" "MultiplyWithRoot" 0 (Utilities|Array|Get(acopy) (.availablepins (Utilities|Array|Get(acopy) (Variables|Default|GetPinSets))) 1) false 0))
      (Variables|Default|SetPlayerPinRing _returnvalue_2))))

(event EventTick
  (params (DeltaSeconds :type Float%20%28single-precision%29))
  (CallFunction|MoveObstacles DeltaSeconds)
  (CallFunction|CycleObstacles))

(fn MovePlayerPins
  (params (Right :type Boolean))
  (Default|Move (Variables|Default|GetPlayerPinRing) Right)
  (bind _fits (Default|CheckPins (Variables|Default|GetActiveIncomingRing) (Variables|Default|GetPlayerPinRing)))
  (if _fits
    (Rendering|Debug|DrawDebugSphere "0, 0, 0" 2e+01 12 "(R=0.155549,G=1.000000,B=0.142031,A=1.000000)" 0.2 1.0)
    (else
      (Rendering|Debug|DrawDebugBox "0, 0, 0" "10.000000,10.000000,10.000000" "(R=1.000000,G=0.049340,B=0.009540,A=1.000000)" "0, 0, 0" 0.2 0.0))))

(fn CycleObstacles
  (bind _updatedobstacles (LocalVariables|GetUpdatedObstacles))
  (Utilities|FlowControl|Sequence
    (:then_0
      (for _array_element (Variables|Default|GetObstacleRings)
        ;[1 1 1] destroy rings that are far enough behind the camera
        (if (< (.x (Transformation|GetActorLocation _array_element)) -5e+02)
          (if (== _array_element (Variables|Default|GetActiveIncomingRing))
            (Variables|Default|SetActiveIncomingRing 0) ; clear it just in case
          )
          (Actor|DestroyActor _array_element)
          (else
            (Utilities|Array|Add (LocalVariables|GetUpdatedObstacles) _array_element) ; it's not behind the camera, add it
          ))))
    (:then_1
      ;[1 1 1] find closest ring to make it the incoming one
      (bind _array_element_2 (Utilities|Array|ForEachLoopwithBreak (LocalVariables|GetUpdatedObstacles) :!label _label)
        (:LoopBody
          (if (>= (.x (Transformation|GetActorLocation _array_element_2)) 0.0)
            (LocalVariables|SetFoundNewIncomingRing _array_element_2)
            (goto _label Break)))
        (:Completed
          (Utilities|IsValid (LocalVariables|GetFoundNewIncomingRing)
            (:Is%20Valid
              (Variables|Default|SetActiveIncomingRing (LocalVariables|GetFoundNewIncomingRing)))
            (:Is%20Not%20Valid
              (Variables|Default|SetActiveIncomingRing 0))))))
    (:then_2
      (if (Utilities|Array|IsNotEmpty _updatedobstacles)
        (LocalVariables|SetLastRingDistance (.x (Transformation|GetActorLocation (Utilities|Array|Get(acopy) _updatedobstacles (Utilities|Array|LastIndex _updatedobstacles)))))))
    (:then_3
      (for _index (range (Utilities|Array|Length (LocalVariables|GetUpdatedObstacles)) 5)
        (bind _returnvalue (Game|SpawnActorfromClass "/Game/Blueprints/ObstacleRing.ObstacleRing_C" (Math|Transform|MakeTransform (Math|Vector|MakeVector (+ (* (Variables|Default|GetRingInterval) _index) (LocalVariables|GetLastRingDistance)) 0.0 0.0) "0, 0, 0" "1.000000,1.000000,1.000000") "AlwaysSpawn" "MultiplyWithRoot" 0 (.OutItem (Utilities|Array|Random (Variables|Default|GetAvailableRings))) true 0))
        (Utilities|Array|Add (LocalVariables|GetUpdatedObstacles) _returnvalue)))
    (:then_4
      (Variables|Default|SetObstacleRings (LocalVariables|GetUpdatedObstacles)))))

(fn MoveObstacles
  (params (DeltaTime :type Float%20%28double-precision%29))
  (for _array_element (Variables|Default|GetObstacleRings)
    (Transformation|AddActorLocalOffset _array_element (Math|Vector|MakeVector (* DeltaTime -2e+02) 0.0 0.0) false false)))