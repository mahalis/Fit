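; JamMode is the game mode for a ring-and-pin arcade game, running the flow from title through play, pause and game over.
; On BeginPlay it creates all UI widgets up front, then toggles their visibility, input modes, mapping contexts and game pause per state.
; It forwards move and switch requests to RingManager.
; Passed rings award doubling points by fitting pin count or cost a life, updating the HUD and ending the game at zero.
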(event EventBeginPlay
  (Utilities|FlowControl|Sequence
    (:then_0
      (CallFunction|CreateUI)
      (Input|AddMappingContext (PlayerController|LocalPlayerSubsystems|GetEnhancedInputLocalPlayerSubsystem (Game|GetPlayerController 0)) "/Game/Input/BaseContext.BaseContext" 0 "(bIgnoreAllPressedKeysUntilRelease=True,bForceImmediately=False,bNotifyUserSettings=False)"))
    (:then_1
      (bind _outactors (Actor|GetAllActorsOfClasswithTag "/Script/Engine.CameraActor" "Main"))
      (Variables|Default|SetMainCamera (Utilities|Array|Get(acopy) _outactors)))
    (:then_2
      (Audio|Components|Audio|Play (Variables|Default|GetMusic) 0.0))
    (:then_3
      (Game|Player|SetViewTargetwithBlend (Game|GetPlayerController 0) (Variables|Default|GetMainCamera) 0.0 "VTBlend_Linear" 0.0 false))
    (:then_4
      (CallFunction|Reset))))

(event EventTick
  (params (DeltaSeconds :type Float%20%28single-precision%29)))

(fn ConstructionScript)

(fn CreateUI
  (bind _returnvalue (Game|GetPlayerController 0))
  (Utilities|FlowControl|Sequence
    (:then_0
      (bind _returnvalue_2 (UserInterface|CreateWidget "/Game/Blueprints/UI/PauseMenuWidget.PauseMenuWidget_C" _returnvalue))
      (bind _output_get (Variables|UI|SetPauseWidget _returnvalue_2))
      (UserInterface|Viewport|AddtoViewport _output_get 1)
      (Widget|SetVisibility _output_get "Hidden"))
    (:then_1
      (bind _returnvalue_3 (UserInterface|CreateWidget "/Game/Blueprints/UI/ScoreHUD.ScoreHUD_C" _returnvalue))
      (bind _output_get_2 (Variables|UI|SetHUDWidget _returnvalue_3))
      (UserInterface|Viewport|AddtoViewport _output_get_2 0)
      (Widget|SetVisibility _output_get_2 "Hidden"))
    (:then_2
      (bind _returnvalue_4 (UserInterface|CreateWidget "/Game/Blueprints/UI/TitleWidget.TitleWidget_C" _returnvalue))
      (bind _output_get_3 (Variables|UI|SetTitleWidget _returnvalue_4))
      (UserInterface|Viewport|AddtoViewport _output_get_3 2)
      (Widget|SetVisibility _output_get_3 "Visible"))
    (:then_3
      (bind _returnvalue_5 (UserInterface|CreateWidget "/Game/Blueprints/UI/GameOverWidget.GameOverWidget_C" _returnvalue))
      (bind _output_get_4 (Variables|UI|SetGameOverWidget _returnvalue_5))
      (UserInterface|Viewport|AddtoViewport _output_get_4 3)
      (Widget|SetVisibility _output_get_4 "Hidden"))))

(fn RequestSetPaused
  (params (Paused :type Boolean))
  (bind _returnvalue (Game|GetPlayerController 0))
  (bind _returnvalue_2 (PlayerController|LocalPlayerSubsystems|GetEnhancedInputLocalPlayerSubsystem _returnvalue))
  (bind _output_get (Variables|Default|SetIsFakePaused Paused))
  (Game|SetGamePaused _output_get)
  (Widget|SetVisibility (Variables|UI|GetPauseWidget) (select _output_get "Visible" "Hidden"))
  (if _output_get
    (Input|RemoveMappingContext _returnvalue_2 "/Game/Input/InGameContext.InGameContext" "(bIgnoreAllPressedKeysUntilRelease=True,bForceImmediately=False,bNotifyUserSettings=False)")
    (Input|SetInputModeUIOnly _returnvalue (Variables|UI|GetPauseWidget) "DoNotLock" false)
    (else
      (Input|AddMappingContext _returnvalue_2 "/Game/Input/InGameContext.InGameContext" 0 "(bIgnoreAllPressedKeysUntilRelease=True,bForceImmediately=False,bNotifyUserSettings=False)")
      (Input|SetInputModeGameOnly _returnvalue true))))

(fn Begin
  (CallFunction|RequestSetPaused false)
  (bind _output_get (Variables|Default|SetCurrentScore 0))
  (Default|UpdateScore (Variables|UI|GetHUDWidget) 0 _output_get)
  (Variables|/Game/Blueprints/RingManagerComponent.RingManagerComponent_C|SetShouldAutoSpawnRings (Variables|Default|GetRingManager) true)
  (Widget|SetVisibility (Variables|UI|GetTitleWidget) "Hidden")
  (Input|AddMappingContext (PlayerController|LocalPlayerSubsystems|GetEnhancedInputLocalPlayerSubsystem (Game|GetPlayerController 0)) "/Game/Input/InGameContext.InGameContext" 0 "(bIgnoreAllPressedKeysUntilRelease=True,bForceImmediately=False,bNotifyUserSettings=False)")
  (Input|SetInputModeGameOnly (Game|GetPlayerController 0) true)
  (Widget|SetVisibility (Variables|UI|GetHUDWidget) "Visible"))

(fn IsPaused
  (return (Variables|Default|GetIsFakePaused)))

(fn RequestMove
  (params (Right :type Boolean))
  (Default|MovePlayerPins (Variables|Default|GetRingManager) Right))

(fn RequestSwitchPins
  (params (Forward :type Boolean))
  (Default|SwitchPlayerPins (Variables|Default|GetRingManager) Forward))

(fn NotifyPassedRing
  (params (Success :type Boolean) (FittingPinCount :type Integer) (Ring :type Obstacle%20Ring%20Object%20Reference))
  (bind _returnvalue (Utilities|Select :Index FittingPinCount :Option%200 0 :Option%201 10 :Option%202 20 :Option%203 40 :Option%204 80))
  (Default|NotifyPassed Ring Success)
  (if Success
    (bind _output_get (Variables|Default|SetCurrentScore (+ (Variables|Default|GetCurrentScore) _returnvalue)))
    (Default|UpdateScore (Variables|UI|GetHUDWidget) _returnvalue _output_get)
    (else
      (CallFunction|DeductLife))))

(fn Reset
  (bind _hudwidget (Variables|UI|GetHUDWidget))
  (bind _titlewidget (Variables|UI|GetTitleWidget))
  (Utilities|FlowControl|Sequence
    (:then_0
      (Game|SetGamePaused true)
      (Variables|Default|SetIsFakePaused true)
      (Widget|SetVisibility _titlewidget "Visible")
      (Input|SetInputModeUIOnly (Game|GetPlayerController 0) _titlewidget "DoNotLock" true))
    (:then_1
      (bind _output_get (Variables|Default|SetCurrentLives (Variables|Default|GetInitialLives)))
      (bind _output_get_2 (Variables|Default|SetCurrentScore 0))
      (Default|UpdateLives _hudwidget _output_get false)
      (Default|UpdateScore _hudwidget 0 _output_get_2))
    (:then_2
      (Default|Reset (Variables|Default|GetRingManager)))))

(fn DeductLife
  (bind _output_get (Variables|Default|SetCurrentLives (- (Variables|Default|GetCurrentLives) 1)))
  (Default|UpdateLives (Variables|UI|GetHUDWidget) _output_get true)
  (if (not (> _output_get 0)) ; still alive?
    (CallFunction|EndGame)))

(fn EndGame
  (bind _gameoverwidget (Variables|UI|GetGameOverWidget))
  (Variables|Default|SetIsFakePaused true)
  (Game|SetGamePaused true)
  (Widget|SetVisibility _gameoverwidget "Visible")
  (Input|SetInputModeUIOnly (Game|GetPlayerController 0) _gameoverwidget "DoNotLock" false))

(fn ReturntoTitleScreen
  (bind _titlewidget (Variables|UI|GetTitleWidget))
  (CallFunction|Reset)
  (Widget|SetVisibility (Variables|UI|GetGameOverWidget) "Hidden")
  (Widget|SetVisibility _titlewidget "Visible")
  (Input|SetInputModeUIOnly (Game|GetPlayerController 0) _titlewidget "DoNotLock" false))