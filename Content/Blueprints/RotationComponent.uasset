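; Rotation component that tracks a stepped offset around a ring of equal segments and holds a spring-smoothed rotation value.
; Move steps the offset one segment either way, while SetOffsetInstant overwrites it directly.
; State converts the unbounded offset into negative-signed degrees and a wrapped segment index, using a large bias to handle negatives.
; Tick spring-interpolates RotationCurrent toward RotationTarget, which no graph here sets.
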(event EventBeginPlay)

(event EventTick
  (params (DeltaSeconds :type Float%20%28single-precision%29))
  (bind _returnvalue (Class|KismetMathLibrary|FloatSpringInterp (Variables|Default|GetRotationCurrent) (Variables|Default|GetRotationTarget) (Variables|Default|GetRotationSpringState) 0.0 0.8 DeltaSeconds 1.0 1.0))
  (Variables|Default|SetRotationCurrent _returnvalue))

(fn Move
  (params (Right :type Boolean))
  (Variables|Default|SetSegmentOffset (+ (Variables|Default|GetSegmentOffset) (Math|Integer|SelectInt 1 -1 Right) 0))
  (return))

(fn State
  (bind _segmentoffset (Variables|Default|GetSegmentOffset))
  (bind _segmentcount (Variables|Default|GetSegmentCount))
  (return (* (/ (Math|Conversions|ToFloat(Integer) _segmentoffset) _segmentcount) -3.6e+02) (Math|Integer|%(Integer) (+ _segmentoffset (* _segmentcount 5000)) _segmentcount)))

(fn SetOffsetInstant
  (params (Offset :type Integer))
  (Variables|Default|SetSegmentOffset Offset))