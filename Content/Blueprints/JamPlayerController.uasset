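; Player controller that turns input actions into game requests for pausing, moving and switching pins.
; On BeginPlay it caches the game mode as JamMode and forwards every action to it, holding no gameplay logic itself.
; Move and switch actions reduce their input value to a positive-or-not boolean, and the pause action inverts the mode's current paused state.
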(event Input|EnhancedActionEvents|EnhancedInputActionTogglePauseAction
  (params (ActionValue :type Boolean) (ElapsedSeconds :type Float%20%28double-precision%29) (TriggeredSeconds :type Float%20%28double-precision%29) (InputAction :type Input%20Action%20Object%20Reference :default "/Game/Input/TogglePauseAction.TogglePauseAction"))
  (bind _mode (Variables|Default|GetMode))
  (Default|RequestSetPaused _mode (not (Default|IsPaused _mode))))

(event Input|EnhancedActionEvents|EnhancedInputActionMoveAction
  (params (ActionValue :type Float%20%28double-precision%29) (ElapsedSeconds :type Float%20%28double-precision%29) (TriggeredSeconds :type Float%20%28double-precision%29) (InputAction :type Input%20Action%20Object%20Reference :default "/Game/Input/MoveAction.MoveAction"))
  (Default|RequestMove (Variables|Default|GetMode) (> ActionValue 0.0)))

(event Input|EnhancedActionEvents|EnhancedInputActionSwitchAction
  (params (ActionValue :type Float%20%28double-precision%29) (ElapsedSeconds :type Float%20%28double-precision%29) (TriggeredSeconds :type Float%20%28double-precision%29) (InputAction :type Input%20Action%20Object%20Reference :default "/Game/Input/SwitchAction.SwitchAction"))
  (Default|RequestSwitchPins (Variables|Default|GetMode) (> ActionValue 0.0)))

(event EventBeginPlay
  (bind _asjam_mode (Utilities|Casting|CastToJamMode (Game|GetGameMode)))
  (Variables|Default|SetMode _asjam_mode))

(event EventTick
  (params (DeltaSeconds :type Float%20%28single-precision%29)))

(fn ConstructionScript)